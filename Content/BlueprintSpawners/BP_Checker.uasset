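; BP_Checker is a Blueprint that spawns a StaticMeshActor at the transform of every AISpawn actor on BeginPlay.
; Each spawned actor is owned by its AISpawn and has collision disabled, while its SetStaticMesh call names no mesh.
; A Distance counter grows with each iteration, but the vertical-offset vector that reads it is unused, so it never affects placement.
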(event `self.ReceiveBeginPlay`
  (bind _outactors (`GameplayStatics.GetAllActorsOfClass` "/Script/ReadyOrNot.AISpawn"))
  (for _array_element _outactors
    (bind _returnvalue (`|SpawnActorFromClass` "/Script/Engine.StaticMeshActor" (`self.GetTransform` _array_element) "AlwaysSpawn" "OverrideRootScale" _array_element null))
    (bind _staticmeshcomponent (`StaticMeshActor.StaticMeshComponent` _returnvalue))
    (`StaticMeshComponent.SetStaticMesh` _staticmeshcomponent null)
    (set `self.distance` (+ (`self.distance`) 50.0))
    (`PrimitiveComponent.SetCollisionEnabled` _staticmeshcomponent "NoCollision")))

(fn `UserConstructionScript`)