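; BP_Door is a level-placed spawner that stands in for a BP_Door_New door at runtime.
; On BeginPlay, the authority spawns BP_Door_New at the same transform, passing along door type, trap, lock, mesh and open-range settings, then destroys itself.
; The construction script hides the preview cube when the selected door type row is Doorway.
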(event `self.ReceiveBeginPlay`
  (`/Engine/EditorBlueprintResources/ActorMacros.Switch Has Authority`
    (:`Authority`
      (`|SpawnActorFromClass` "/Game/Blueprints/Environment/BP_Door_New.BP_Door_New_C" (`self.GetTransform`) "Undefined" "OverrideRootScale" null (`self.Door Type`) (`self.Trap Type`) (`self.CanLock`) (`self.Lock Chance`) (`self.bUseBrokenDoorMesh`) (`self.MinOpen`) (`self.MaxOpen`) (`self.NoSpawnTrap`) null)
      (`self.K2_DestroyActor`))))

(fn `UserConstructionScript`
  (bind _cube1 (`self.Cube1`))
  (if (== (`.RowName` (break `DataTableRowHandle` (`self.Door Type`))) "Doorway")
    (`SceneComponent.SetVisibility` _cube1 false true)
    (else
      (`SceneComponent.SetVisibility` _cube1 true true))))