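; BP_SpawnAI is a placeable randomizer that spawns an AISpawner at its transform on BeginPlay, with a random enabled state.
; It is suspect or civilian at random unless OverrideSus keeps the OnlySus setting.
; Unless a data table override is set, it builds the AI row handle from separate random rolls for roster table and row-name list, so the two can mismatch.
; The construction script sets a suspect or civilian billboard sprite from OnlySus.
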(event `self.ReceiveBeginPlay`
  (bind _returnvalue (`KismetMathLibrary.RandomIntegerInRange` 0 5))
  (set `self.OnlySus` (select `bool` (`self.Override Sus`) :`false` (`KismetMathLibrary.RandomBool`) :`true` (`self.OnlySus`)))
  (`|SpawnActorFromClass` "/Game/Blueprints/Logic/AISpawner.AISpawner_C" (`self.GetTransform`) "AlwaysSpawn" "OverrideRootScale" null (`KismetMathLibrary.RandomBool`) (select `bool` (`self.Override DataTablesStruct`) :`false` (make `DataTableRowHandle` (select `int` _returnvalue :`0` "/Game/Blueprints/DataTables/AIDataTable.AIDataTable" :`1` "/Game/Blueprints/DataTables/AI/AIDataTable_Dealer.AIDataTable_Dealer" :`2` "/Game/Blueprints/DataTables/AI/AIDataTable_Gas.AIDataTable_Gas" :`3` "/Game/Blueprints/DataTables/AI/AIDataTable_Hotel.AIDataTable_Hotel" :`4` "/Game/Blueprints/DataTables/AI/AIDataTable_Meth.AIDataTable_Meth" :`5` "/Game/Blueprints/DataTables/AIDataTable_V3.AIDataTable_V3" :!type "DataTable Object Reference") (`KismetArrayLibrary.Array_Random` (select `bool` (`self.OnlySus`) :`false` (select `int` _returnvalue :`0` (`|MakeArray` "Civilian_NewMeth_03" "Civilians_HotelRoster_GuestsMale" "Civilian_Gas_Roster_Sharla" :!type "Name") :`1` (`|MakeArray` "cv_m_dealer_salesman_lead" "cv_m_dealer_salesman" :!type "Name") :`2` (`|MakeArray` "Civilian_Gas_Woman_01" "Civilian_Gas_Hobo" "Civilian_Gas_Employee_01" "Civilian_Hotel_Civilian_Chef" "Civilian_Hotel_Civilian_Chef_Executive" "Civilian_Hotel_Civilian_Man_02" "Civilian_Hotel_Civilian_Man_04" "Civilian_Gas_Employee_02" "Civilian_Gas_Employee_03" "Civilian_Gas_Autoparts_01" :!type "Name") :`3` (`|MakeArray` "cv_f_hotel_employee" "cv_m_construction" "cv_m_guest" "cv_f_belle" :!type "Name") :`4` (`|MakeArray` "cv_f_meth_01" "cv_f_meth_02" "cv_m_meth_01" :!type "Name") :`5` (`|MakeArray` "Civilian_NewClub_01F" "Civilian_NewClub_01M" :!type "Name")) :`true` (select `int` _returnvalue :`0` (`|MakeArray` "Suspect_AliDevTest_01" "Suspects_Cult_Suspect_01" "Suspect_NewMeth_2F_shotgunner" "Suspect_NewClub_L1NoGun" "Suspects_HotelRoster_LLP_L1" "Suspects_HotelRoster_LLP_L2" "Suspects_HotelRoster_LLP_L3" "Suspects_HotelRoster_LLP_Leader" "Suspects_GasRoster_Zion" :!type "Name") :`1` (`|MakeArray` "sp_m_dealer_mechanic" "sp_m_dealer_salesman" "sp_m_dealer_salesman_lead" :!type "Name") :`2` (`|MakeArray` "Suspect_01_Shotgun" "Suspect_02_Pistol" "Suspect_03_Revolver" "Suspect_04_Pistol" "Suspect_ActiveShooter" :!type "Name") :`3` (`|MakeArray` "sp_m_shooter_a" "cs_m_hotel_employee" "sp_m_shooter_b" "sp_m_shooter_c" :!type "Name") :`4` (`|MakeArray` "sp_f_meth" "sp_m_meth" "sp_m_meth_02" :!type "Name") :`5` (`|MakeArray` "Suspect_NewClub_L3Zahir" "Suspect_NewClub_L2Shotgun" "Suspect_NewClub_L2Assault" "Suspect_NewClub_L1Pistol" "Suspect_NewClub_L1Uzi" "Suspect_NewClub_L2Assault_Armor" "Suspect_NewClub_L2Shotgun_Armor" "Suspect_NewClub_L3Heavy" :!type "Name"))))) :`true` (`self.AI Datatable`)) null))

(fn `UserConstructionScript`
  (`BillboardComponent.SetSprite` (`self.Billboard`) (select `bool` (`self.OnlySus`) :`false` "/Game/ReadyOrNot/UI/Elements/CivSpawn.CivSpawn" :`true` "/Game/ReadyOrNot/UI/Elements/SusSpawn.SusSpawn" :!type "Texture2D Object Reference")))